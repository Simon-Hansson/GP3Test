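; Actor component that lets the third-person player character glide while IA_Glide is held, starting once downward velocity passes a threshold.
; Each trigger lerps velocity toward a set vertical speed and forward horizontal speed, while a DoOnce zeroes gravity and falling braking.
; Turn rate changes on press; release or cancel restores movement using hard-coded values, leaving the defaults cached at BeginPlay unused.
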(event `self.ReceiveBeginPlay`
  (bind _asbp_third_person_character (cast `/Game/ThirdPerson/Blueprints/BP_ThirdPersonCharacter` (`GameplayStatics.GetPlayerCharacter` 0)))
  (bind _output_get (set `self.As BP Third Person Character` _asbp_third_person_character))
  (set `self.Character Movement Component` (`Character.CharacterMovement` _output_get))
  (set `self.Default Braking Deceleration` (`CharacterMovementComponent.BrakingDecelerationFalling` (`self.Character Movement Component`)))
  (set `self.Default Air Control` (`CharacterMovementComponent.AirControl` (`self.Character Movement Component`)))
  (set `self.Default Air Control Boost Multiplier` (`CharacterMovementComponent.AirControlBoostMultiplier` (`self.Character Movement Component`)))
  (set `self.Default Air Control Boost Velocity Threshold` (`CharacterMovementComponent.AirControlBoostVelocityThreshold` (`self.Character Movement Component`))))

(event `EnhancedInput|/Game/Input/Actions/IA_Glide`
  (params (ActionValue :type Boolean) (ElapsedSeconds :type "Float (double-precision)") (TriggeredSeconds :type "Float (double-precision)") (InputAction :type "InputAction Object Reference" :default "/Game/Input/Actions/IA_Glide.IA_Glide"))
  (bind (_returnvalue_x _returnvalue_y _returnvalue_z) (`KismetMathLibrary.BreakVector` (`NavMovementComponent.GetVelocityForNavMovement` (`self.Character Movement Component`))))
  ; Glide logic. Hold space for 0.3 seconds (edited in AI_Glide Input Asset) to trigger. Can only glide if character is moving downwards.
  (:`Triggered`
    (if (< _returnvalue_z -650.0)
      (set `/Game/ThirdPerson/Blueprints/BP_ThirdPersonCharacter.IsGliding` true (`self.As BP Third Person Character`))
      (bind _verticalspeed (`self.LerpVerticalSpeed` :!label _label))
      (bind (_returnvalue_x_2 _returnvalue_y_2) (`self.LerpHorizontalSpeed`))
      (set `MovementComponent.Velocity` (`KismetMathLibrary.MakeVector` _returnvalue_x_2 _returnvalue_y_2 _verticalspeed) (`self.Character Movement Component`))
      (`/Engine/EditorBlueprintResources/StandardMacros.DoOnce` false :!label _label_2
        (:`Completed`
          (set `CharacterMovementComponent.GravityScale` 0.0 (`self.Character Movement Component`))
          (set `CharacterMovementComponent.BrakingDecelerationFalling` 0.0 (`self.Character Movement Component`))))
      (elif (`/Game/ThirdPerson/Blueprints/BP_ThirdPersonCharacter.IsGliding` (`self.As BP Third Person Character`))
        (goto _label))))
  (:`Started`
    (set `CharacterMovementComponent.RotationRate` (`self.GlideTurnSpeed`) (`self.Character Movement Component`)))
  (:`Canceled`
    (set `CharacterMovementComponent.GravityScale` 1.5 (`self.Character Movement Component`) :!label _label_3)
    (set `CharacterMovementComponent.BrakingDecelerationFalling` 250.0 (`self.Character Movement Component`))
    (set `CharacterMovementComponent.bOrientRotationToMovement` true (`self.Character Movement Component`))
    (set `/Game/ThirdPerson/Blueprints/BP_ThirdPersonCharacter.IsGliding` false (`self.As BP Third Person Character`))
    (set `CharacterMovementComponent.RotationRate` (struct :`Yaw` 500.0) (`self.Character Movement Component`))
    (goto _label_2 :!via `Reset`))
  (:`Completed`
    (goto _label_3)))

(fn `LerpHorizontalSpeed`
  (returns (ReturnValue_X :type "Float (double-precision)") (ReturnValue_Y :type "Float (double-precision)"))
  (bind _horizontalglidespeed (`self.HorizontalGlideSpeed`))
  (bind (_returnvalue_x _returnvalue_y) (`KismetMathLibrary.BreakVector` (`KismetMathLibrary.VLerp` (`Actor.GetVelocity` (`self.As BP Third Person Character`)) (* (`Actor.GetActorForwardVector` (`self.As BP Third Person Character`)) (`KismetMathLibrary.MakeVector` _horizontalglidespeed _horizontalglidespeed _horizontalglidespeed)) (`self.Acceleration`))))
  (return _returnvalue_x _returnvalue_y))

(fn `LerpVerticalSpeed`
  (returns (VerticalSpeed :type "Float (double-precision)"))
  (bind (_returnvalue_x _returnvalue_y _returnvalue_z) (`KismetMathLibrary.BreakVector` (`NavMovementComponent.GetVelocityForNavMovement` (`self.Character Movement Component`))))
  (return (`KismetMathLibrary.Lerp` _returnvalue_z (`self.VerticalGlideSpeed`) (`self.LerpVerticalGlideSpeed`))))