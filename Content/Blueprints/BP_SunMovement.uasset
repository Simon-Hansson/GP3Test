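; BP_SunMovement animates a referenced directional light to move the sun across the sky.
; Looping timers step the light's pitch up or down between limits while yaw always advances, starting with the upward move.
; On reaching a limit, FlipSunMovement clears both timers and chooses the next direction from the current pitch.
; Each step copies the light's rotation to SunRotation on the player's BP_ThirdPersonCharacter.
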(event `self.ReceiveBeginPlay`
  (`|ExecutionSequence`
    (:`then_0`
      (`self.InitializeSunMovement`))
    (:`then_1`
      (bind _asbp_third_person_character (cast `/Game/ThirdPerson/Blueprints/BP_ThirdPersonCharacter` (`GameplayStatics.GetPlayerCharacter` 0)))
      (set `self.As BP Third Person Character` _asbp_third_person_character))))

(event `MoveSunUp`
  (bind (_returnvalue_roll _returnvalue_pitch _returnvalue_yaw) (`KismetMathLibrary.BreakRotator` (`self.K2_GetActorRotation` (`self.Directional Light Ref`))))
  (set `self.CurrentSunY` _returnvalue_pitch)
  (set `self.CurrentSunZ` _returnvalue_yaw)
  (if (>= (`self.CurrentSunY`) (`self.MaxSunY`))
    (`self.K2_SetActorRotation` (`self.Directional Light Ref`) (`KismetMathLibrary.MakeRotator` 0.0 (- (`self.CurrentSunY`) (`self.VerticalStepDistance`)) (+ (`self.CurrentSunZ`) (`self.HorizontalStepDistance`))) false)
    (set `/Game/ThirdPerson/Blueprints/BP_ThirdPersonCharacter.Sun Rotation` (`self.K2_GetActorRotation` (`self.Directional Light Ref`)) (`self.As BP Third Person Character`))
    (else
      (`self.FlipSunMovement`))))

(event `MoveSunDown`
  (bind (_returnvalue_roll _returnvalue_pitch _returnvalue_yaw) (`KismetMathLibrary.BreakRotator` (`self.K2_GetActorRotation` (`self.Directional Light Ref`))))
  (set `self.CurrentSunY` _returnvalue_pitch)
  (set `self.CurrentSunZ` _returnvalue_yaw)
  (if (<= (`self.CurrentSunY`) (`self.MinSunY`))
    (`self.K2_SetActorRotation` (`self.Directional Light Ref`) (`KismetMathLibrary.MakeRotator` 0.0 (+ (`self.CurrentSunY`) (`self.VerticalStepDistance`)) (+ (`self.CurrentSunZ`) (`self.HorizontalStepDistance`))) false)
    (set `/Game/ThirdPerson/Blueprints/BP_ThirdPersonCharacter.Sun Rotation` (`self.K2_GetActorRotation` (`self.Directional Light Ref`)) (`self.As BP Third Person Character`))
    (else
      (`self.FlipSunMovement`))))

(event `FlipSunMovement`
  (`|ExecutionSequence`
    (:`then_0`
      (if (`KismetSystemLibrary.K2_IsValidTimerHandle` (`self.MoveSunUpTimerHandle`))
        (`KismetSystemLibrary.K2_ClearAndInvalidateTimerHandle` (`self.MoveSunUpTimerHandle`))))
    (:`then_1`
      (if (`KismetSystemLibrary.K2_IsValidTimerHandle` (`self.MoveSunDownTimerHandle`))
        (`KismetSystemLibrary.K2_ClearAndInvalidateTimerHandle` (`self.MoveSunDownTimerHandle`))))
    (:`then_2`
      (if (>= (`self.CurrentSunY`) (`self.MinSunY`))
        (bind _returnvalue (`KismetSystemLibrary.K2_SetTimerDelegate` (`|CreateDelegate` :!event `MoveSunUp`) (`self.TickSpeed`) true :!label _label))
        (set `self.MoveSunUpTimerHandle` _returnvalue)
        (else
          (bind _returnvalue_2 (`KismetSystemLibrary.K2_SetTimerDelegate` (`|CreateDelegate` :!event `MoveSunDown`) (`self.TickSpeed`) true))
          (set `self.MoveSunDownTimerHandle` _returnvalue_2))))))

(event `InitializeSunMovement`
  (goto _label))

(fn `UserConstructionScript`)