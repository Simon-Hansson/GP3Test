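; Battery component for BP_ThirdPersonCharacter that tracks a capacity, starting full, which charges or drains with the character's charging state.
; It binds to the character's ACShadowDetector charging and draining events on BeginPlay.
; Looping timers step capacity up or down at separate tick rates, with each mode clearing the other's timer.
; Battery full and empty events fire when a tick finds capacity at its limit.
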(event `self.ReceiveBeginPlay`
  (set `self.CurrentCapacity` (`self.MaxCapacity`))
  (`|ExecutionSequence`
    (:`then_0`
      (bind _asbp_third_person_character (cast `/Game/ThirdPerson/Blueprints/BP_ThirdPersonCharacter` (`self.GetOwner`)))
      (set `self.As BP Third Person Character` _asbp_third_person_character))
    (:`then_1`
      (add `/Game/Blueprints/AC_ShadowDetector.OnIsCharging` (`/Game/ThirdPerson/Blueprints/BP_ThirdPersonCharacter.AC_ShadowDetector` (`self.As BP Third Person Character`)) (`|CreateDelegate` :!event `DoBatteryStuff`)))
    (:`then_2`
      (add `/Game/Blueprints/AC_ShadowDetector.OnIsDraining` (`/Game/ThirdPerson/Blueprints/BP_ThirdPersonCharacter.AC_ShadowDetector` (`self.As BP Third Person Character`)) (`|CreateDelegate` :!event `DoBatteryStuff`)))))

(event `DoBatteryStuff`
  (if (`/Game/ThirdPerson/Blueprints/BP_ThirdPersonCharacter.Is Charging` (`self.As BP Third Person Character`))
    (bind _returnvalue (`KismetSystemLibrary.K2_SetTimerDelegate` (`|CreateDelegate` :!event `ChargeBattery`) (`self.ChargeTickSpeed`) true))
    (set `self.ChargeTimerHandle` _returnvalue)
    (`KismetSystemLibrary.K2_ClearAndInvalidateTimerHandle` (`self.DrainTimerHandle`))
    (else
      (bind _returnvalue_2 (`KismetSystemLibrary.K2_SetTimerDelegate` (`|CreateDelegate` :!event `DrainBattery`) (`self.DrainTickSpeed`) true))
      (set `self.DrainTimerHandle` _returnvalue_2)
      (`KismetSystemLibrary.K2_ClearAndInvalidateTimerHandle` (`self.ChargeTimerHandle`)))))

(event `ChargeBattery`
  (if (< (`self.CurrentCapacity`) (`self.MaxCapacity`))
    (`/Engine/EditorBlueprintResources/StandardMacros.IncrementFloat` (`self.CurrentCapacity`))
    (else
      (`self.OnBatteryFull`))))

(event `DrainBattery`
  (if (> (`self.CurrentCapacity`) 0.0)
    (`/Engine/EditorBlueprintResources/StandardMacros.DecrementFloat` (`self.CurrentCapacity`))
    (else
      (`self.OnBatteryEmpty`))))