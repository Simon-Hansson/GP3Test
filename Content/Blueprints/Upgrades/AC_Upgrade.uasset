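; Actor component that applies upgrades to the player's battery component, AC_Battery, which it fetches from the player character on BeginPlay.
; DoUpgrade switches on the upgrade type, steps one battery stat by a fixed amount while within its cap, and prints it.
; Case names do not match their stats: Tick Amount raises MaxCapacity, Drain Amount lowers ChargeTickSpeed, Max Capacity raises DrainTickSpeed.
; The upgrade's Value is stored but never applied.
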(event `self.ReceiveBeginPlay`
  (set `self.AC_Battery` (`Actor.GetComponentByClass` (`GameplayStatics.GetPlayerCharacter` 0) "/Game/Blueprints/AC_Battery.AC_Battery_C")))

(event `/Game/Blueprints/Upgrades/BPI_DoUpgrade.DoUpgrade`
  (params (Upgrade :type "/Game/Blueprints/Upgrades/F_Upgrade Structure"))
  (bind _ac_battery (`self.AC_Battery`))
  (bind _ac_battery_2 (`self.AC_Battery`))
  (bind _ac_battery_3 (`self.AC_Battery`))
  (bind _maxcapacity (`/Game/Blueprints/AC_Battery.MaxCapacity` _ac_battery))
  (bind _chargetickspeed (`/Game/Blueprints/AC_Battery.ChargeTickSpeed` _ac_battery_2))
  (bind _draintickspeed (`/Game/Blueprints/AC_Battery.DrainTickSpeed` _ac_battery_3))
  (set `self.Upgrade Name` Upgrade_Type_16_8A30A4274E03AB1256BFC4906D021146)
  (set `self.Upgrade Value` Upgrade_Value_14_2F03BDD94EBA5C62C7412C9FA1E930C7)
  (switch `name` (`self.Upgrade Name`)
    (:`TickAmount`
      (if (< _maxcapacity (`self.MaxCapacityCap`))
        (bind _output_get (set `/Game/Blueprints/AC_Battery.MaxCapacity` (+ _maxcapacity (`self.MaxCapacityUpgradeAmount`)) _ac_battery))
        (`KismetSystemLibrary.PrintString` (`KismetStringLibrary.Conv_DoubleToString` _output_get))))
    (:`DrainAmount`
      (if (> _chargetickspeed (`self.ChargeTickSpeedCap`))
        (bind _output_get_2 (set `/Game/Blueprints/AC_Battery.ChargeTickSpeed` (- _chargetickspeed (`self.ChargeTickSpeedUpgradeAmount`)) _ac_battery_2))
        (`KismetSystemLibrary.PrintString` (`KismetStringLibrary.Conv_DoubleToString` _output_get_2))))
    (:`MaxCapacity`
      (if (< _draintickspeed (`self.DrainTickSpeedCap`))
        (bind _output_get_3 (set `/Game/Blueprints/AC_Battery.DrainTickSpeed` (+ _draintickspeed (`self.DrainTickSpeedUpgradeAmount`)) _ac_battery_3))
        (`KismetSystemLibrary.PrintString` (`KismetStringLibrary.Conv_DoubleToString` _output_get_3))))))