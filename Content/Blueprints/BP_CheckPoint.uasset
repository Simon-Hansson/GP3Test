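; Checkpoint actor that updates the player character's respawn state when its trigger volume is overlapped.
; On BeginPlay it caches the player's BP_ThirdPersonCharacter.
; An overlap writes the RespawnLocation component's world location and relative rotation to that character, plus a sun rotation built from the referenced sun movement actor's current values.
; The overlapping actor is not filtered, as the player comparison is left unconnected.
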(event `self.ReceiveBeginPlay`
  (bind _asbp_third_person_character (cast `/Game/ThirdPerson/Blueprints/BP_ThirdPersonCharacter` (`GameplayStatics.GetPlayerCharacter` 0)))
  (set `self.As BP Third Person Character` _asbp_third_person_character))

(event `self.CheckPointTrigger.OnComponentBeginOverlap`
  (params (OverlappedComponent :type "PrimitiveComponent Object Reference") (OtherActor :type "Actor Object Reference") (OtherComp :type "PrimitiveComponent Object Reference") (OtherBodyIndex :type Integer) (bFromSweep :type Boolean) (SweepResult :type "HitResult Structure (by ref)"))
  (bind _bp_sunmovementref (`self.BP_SunMovementRef`))
  (if true
    (set `/Game/ThirdPerson/Blueprints/BP_ThirdPersonCharacter.RespawnLocation` (`SceneComponent.K2_GetComponentLocation` (`self.RespawnLocation`)) (`self.As BP Third Person Character`))
    (set `/Game/ThirdPerson/Blueprints/BP_ThirdPersonCharacter.RespawnRotation` (`SceneComponent.RelativeRotation` (`self.RespawnLocation`)) (`self.As BP Third Person Character`))
    (bind _output_get (set `self.SunRotation` (`KismetMathLibrary.MakeRotator` 0.0 (`/Game/Blueprints/BP_SunMovement.CurrentSunY` _bp_sunmovementref) (`/Game/Blueprints/BP_SunMovement.CurrentSunZ` _bp_sunmovementref))))
    (set `/Game/ThirdPerson/Blueprints/BP_ThirdPersonCharacter.RespawnSunLocation` _output_get (`self.As BP Third Person Character`))))

(fn `UserConstructionScript`)