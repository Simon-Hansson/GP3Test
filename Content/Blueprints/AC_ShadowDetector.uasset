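; Shadow detection component that decides whether the player's third-person character is charging in sunlight or draining in shade.
; Each tick it derives a distant sun point from the character's SunRotation and runs debug-drawn visibility traces to both foot markers.
; Both traces hitting clears the character's IsCharging; otherwise it is set.
; Paired DoOnce nodes reset each other so OnIsDraining and OnIsCharging dispatchers fire once per state change.
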(event `self.ReceiveBeginPlay`
  (bind _asbp_third_person_character (cast `/Game/ThirdPerson/Blueprints/BP_ThirdPersonCharacter` (`GameplayStatics.GetPlayerCharacter` 0)))
  (set `self.As BP Third Person Character` _asbp_third_person_character))

(event `self.ReceiveTick`
  (params (DeltaSeconds :type "Float (single-precision)"))
  (set `self.SunLocation` (* (`KismetMathLibrary.GetForwardVector` (`/Game/ThirdPerson/Blueprints/BP_ThirdPersonCharacter.Sun Rotation` (`self.As BP Third Person Character`))) (-1000000.0 -1000000.0 -1000000.0)))
  (`|ExecutionSequence`
    (:`then_0`
      (bind (_outhit _returnvalue) (`KismetSystemLibrary.LineTraceSingle` :`Start` (`self.SunLocation`) :`End` (`SceneComponent.K2_GetComponentLocation` (`/Game/ThirdPerson/Blueprints/BP_ThirdPersonCharacter.LeftFootShadowDetection` (`self.As BP Third Person Character`))) :`TraceChannel` "TraceTypeQuery1" :`DrawDebugType` "ForOneFrame"))
      (set `self.IsLeftHit` _returnvalue))
    (:`then_1`
      (bind (_outhit_2 _returnvalue_2) (`KismetSystemLibrary.LineTraceSingle` :`Start` (`self.SunLocation`) :`End` (`SceneComponent.K2_GetComponentLocation` (`/Game/ThirdPerson/Blueprints/BP_ThirdPersonCharacter.RightFootShadowDetection` (`self.As BP Third Person Character`))) :`TraceChannel` "TraceTypeQuery1" :`DrawDebugType` "ForOneFrame"))
      (set `self.IsRightHit` _returnvalue_2)))
  (if (and (`self.IsRightHit`) (`self.IsLeftHit`))
    (set `/Game/ThirdPerson/Blueprints/BP_ThirdPersonCharacter.Is Charging` false (`self.As BP Third Person Character`))
    (`|ExecutionSequence`
      (:`then_0`
        (`/Engine/EditorBlueprintResources/StandardMacros.DoOnce` false :!label _label
          (:`Completed`
            (`self.OnIsDraining`))))
      (:`then_1`
        (goto _label_2 :!via `Reset`)))
    (else
      (set `/Game/ThirdPerson/Blueprints/BP_ThirdPersonCharacter.Is Charging` true (`self.As BP Third Person Character`))
      (`|ExecutionSequence`
        (:`then_0`
          (`/Engine/EditorBlueprintResources/StandardMacros.DoOnce` false :!label _label_2
            (:`Completed`
              (`self.OnIsCharging`))))
        (:`then_1`
          (goto _label :!via `Reset`))))))