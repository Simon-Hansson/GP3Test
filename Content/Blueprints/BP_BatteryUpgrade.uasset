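; BP_BatteryUpgrade is an overlap-triggered upgrade that improves the player character's battery component.
; On BeginPlay it caches the ThirdPerson character and its ACBattery.
; When that character enters the sphere, each enabled flag raises max capacity, lowers charge tick interval or raises drain tick interval by a set amount if its cap is not yet reached, then calls DoBatteryStuff.
; The actor is not destroyed, so re-entering applies upgrades again.
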(event `self.ReceiveBeginPlay`
  (bind _asbp_third_person_character (cast `/Game/ThirdPerson/Blueprints/BP_ThirdPersonCharacter` (`GameplayStatics.GetPlayerCharacter` 0)))
  (bind _output_get (set `self.As BP Third Person Character` _asbp_third_person_character))
  (set `self.AC Battery` (`/Game/ThirdPerson/Blueprints/BP_ThirdPersonCharacter.AC_Battery` _output_get)))

(event `self.Sphere.OnComponentBeginOverlap`
  (params (OverlappedComponent :type "PrimitiveComponent Object Reference") (OtherActor :type "Actor Object Reference") (OtherComp :type "PrimitiveComponent Object Reference") (OtherBodyIndex :type Integer) (bFromSweep :type Boolean) (SweepResult :type "HitResult Structure (by ref)"))
  (bind _ac_battery (`self.AC Battery`))
  (bind _ac_battery_2 (`self.AC Battery`))
  (bind _ac_battery_3 (`self.AC Battery`))
  (bind _maxcapacity (`/Game/Blueprints/AC_Battery.MaxCapacity` _ac_battery))
  (bind _chargetickspeed (`/Game/Blueprints/AC_Battery.ChargeTickSpeed` _ac_battery_3))
  (bind _draintickspeed (`/Game/Blueprints/AC_Battery.DrainTickSpeed` _ac_battery_2))
  (if (== OtherActor (`self.As BP Third Person Character`))
    (`|ExecutionSequence`
      (:`then_0`
        (if (and (`self.MaxCapacityUpgrade`) (< _maxcapacity (`self.MaxCapacityCap`)))
          (set `/Game/Blueprints/AC_Battery.MaxCapacity` (+ _maxcapacity (`self.MaxCapacityUpgradeAmount`)) _ac_battery)
          (`/Game/Blueprints/AC_Battery.DoBatteryStuff` (`self.AC Battery`))))
      (:`then_1`
        (if (and (`self.ChargeTickSpeedUpgrade`) (> _chargetickspeed (`self.ChargeTickSpeedCap`)))
          (set `/Game/Blueprints/AC_Battery.ChargeTickSpeed` (- _chargetickspeed (`self.ChargeTickSpeedUpgradeAmount`)) _ac_battery_3)
          (`/Game/Blueprints/AC_Battery.DoBatteryStuff` (`self.AC Battery`))))
      (:`then_2`
        (if (and (`self.DrainTickSpeedUpgrade`) (< _draintickspeed (`self.DrainTickSpeedCap`)))
          (set `/Game/Blueprints/AC_Battery.DrainTickSpeed` (+ _draintickspeed (`self.DrainTickSpeedUpgradeAmount`)) _ac_battery_2)
          (`/Game/Blueprints/AC_Battery.DoBatteryStuff` (`self.AC Battery`)))))))

(fn `UserConstructionScript`)